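; BP_playerProjectile is a player-fired physics projectile that damages one assigned enemy and destroys itself five seconds after spawning.
; LaunchatEnemy stores that enemy and applies an impulse to the sphere along a supplied forward vector.
; When a second sphere overlaps that enemy, physics stops, CurrentHealth drops by Damage directly and the actor destroys itself shortly after.
; The RecieveDamage call with hitstun and knockback is unconnected, and the Launch event is empty.
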(event OnComponentBeginOverlap(Sphere1)
  (params (OverlappedComponent :type Primitive%20Component%20Object%20Reference) (OtherActor :type Actor%20Object%20Reference) (OtherComp :type Primitive%20Component%20Object%20Reference) (OtherBodyIndex :type Integer) (bFromSweep :type Boolean) (SweepResult :type Hit%20Result%20Structure%20%28by%20ref%29))
  (bind _newvar_0 (Variables|Default|GetNewVar_0))
  (if (== OtherActor _newvar_0)
    (Physics|SetSimulatePhysics (Variables|Default|GetSphere) false)
    (Variables|/Game/Blueprints/CharacterBP/bp_baseCharacter.bp_baseCharacter_C|SetcurrentHealth _newvar_0 (- (Variables|/Game/Blueprints/CharacterBP/bp_baseCharacter.bp_baseCharacter_C|GetcurrentHealth _newvar_0) (Variables|Default|GetDamage)))
    (Utilities|FlowControl|Delay 0.5)
    (CallFunction|DESTROY)))

(event Custom|Launch
  (params (NewParam :type Base%20Player%20BP%20Object%20Reference) (NewParam2 :type Boolean)))

(event EventBeginPlay
  (Utilities|FlowControl|Delay 5.0)
  (Actor|DestroyActor))

(event Collision|EventActorBeginOverlap
  (params (OtherActor :type Actor%20Object%20Reference)))

(event EventTick
  (params (DeltaSeconds :type Float%20%28single-precision%29)))

(fn ConstructionScript)

(fn LaunchatEnemy
  (params (P_ForwardVector :type Vector) (Enemy :type Base%20Player%20BP%20Object%20Reference) (Enemey2 :type Bp%20Base%20Character%20Object%20Reference))
  (Variables|Default|SetNewVar_0 Enemey2)
  (Physics|AddImpulse (Variables|Default|GetSphere) (* P_ForwardVector (Variables|Default|GetlaunchPower)) "None" false))

(fn DESTROY
  (Actor|DestroyActor))