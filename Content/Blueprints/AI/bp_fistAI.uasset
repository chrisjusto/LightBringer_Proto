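; AI controller that fights as a bp_baseCharacter against its Enemy in a melee and projectile combat game.
; Each Tick it either queues a NextAction, picked from the enemy's or its own combat state with random variation, or executes the queued one through the character's functions.
; Knockdowns trigger a randomly delayed get-up.
; An older decision tree, random movement and the timeline feeding the face-enemy gate are disconnected.
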(event Custom|setrotation
  (bind _user (Variables|Default|GetUser))
  (bind _returnvalue (Transformation|GetActorLocation _user))
  (bind _enemy (Variables|/Game/Blueprints/CharacterBP/bp_baseCharacter.bp_baseCharacter_C|GetEnemy _user))
  (bind _returnvalue_2 (Transformation|GetActorLocation _enemy))
  (bind _returnvalue_3 (Math|Rotator|FindLookatRotation _returnvalue _returnvalue_2))
  (bind (_roll _pitch _yaw) (Math|Rotator|BreakRotator _returnvalue_3))
  ;[1 1 1] always look at player
  (Utilities|FlowControl|Gate true) ; enters at Toggle
)

(event EventBeginPlay
  (bind _asbp_base_character (Utilities|Casting|CastTobp_baseCharacter (Pawn|GetControlledPawn)))
  (bind _output_get (Variables|Default|SetUser _asbp_base_character))
  (CallFunction|Setrotation)
  (Variables|/Game/Blueprints/CharacterBP/bp_baseCharacter.bp_baseCharacter_C|SettargetLocked? _output_get true))

(event EventTick
  (params (DeltaSeconds :type Float%20%28single-precision%29))
  (bind _user (Variables|Default|GetUser))
  (bind _user_2 (Variables|Default|GetUser))
  (bind _user_3 (Variables|Default|GetUser))
  (bind _user_4 (Variables|Default|GetUser))
  (bind _user_5 (Variables|Default|GetUser))
  (bind _user_6 (Variables|Default|GetUser))
  (bind _enemy (Variables|/Game/Blueprints/CharacterBP/bp_baseCharacter.bp_baseCharacter_C|GetEnemy _user_2))
  ;[1 1 1] is Valid
  (Utilities|IsValid _user
    (:Is%20Valid
      (Utilities|IsValid (Variables|/Game/Blueprints/CharacterBP/bp_baseCharacter.bp_baseCharacter_C|GetEnemy _user)
        (:Is%20Valid
          (bind _true (Default|KnockedDownCheck (Variables|Default|GetUser)))
          (if (not _true)
            (if (Utilities|Enum|Equal(Enum) (Variables|Default|GetnextAction) "NewEnumerator0")
              (if (Utilities|Enum|Equal(Enum) (Variables|/Game/Blueprints/CharacterBP/bp_baseCharacter.bp_baseCharacter_C|GetcurrentState (Variables|Default|GetUser)) "NewEnumerator0")
                (if (not (Utilities|Enum|Equal(Enum) (Variables|/Game/Blueprints/CharacterBP/bp_baseCharacter.bp_baseCharacter_C|GetcurrentState (Variables|/Game/Blueprints/CharacterBP/bp_baseCharacter.bp_baseCharacter_C|GetEnemy (Variables|Default|GetUser))) "NewEnumerator0"))
                  (switch Utilities|FlowControl|Switch|SwitchonStates (Variables|/Game/Blueprints/CharacterBP/bp_baseCharacter.bp_baseCharacter_C|GetcurrentState (Variables|/Game/Blueprints/CharacterBP/bp_baseCharacter.bp_baseCharacter_C|GetEnemy (Variables|Default|GetUser)))
                    (:NewEnumerator4
                      (if (Variables|/Game/Blueprints/CharacterBP/bp_baseCharacter.bp_baseCharacter_C|GetAttackSnap_inRange _enemy)
                        (Variables|Default|SetnextAction "NewEnumerator3")
                        (else
                          (Variables|Default|SetnextAction "NewEnumerator5"))))
                    (:NewEnumerator6
                      (if (Variables|/Game/Blueprints/CharacterBP/bp_baseCharacter.bp_baseCharacter_C|GetDashSnap_inRange _enemy)
                        (Variables|Default|SetnextAction "NewEnumerator8")
                        (else
                          (switch int (Math|Random|RandomIntegerinRange 0 3)
                            (:0
                              (Variables|/Game/Blueprints/CharacterBP/bp_baseCharacter.bp_baseCharacter_C|SetdashInput _user_2 "NewEnumerator1"))
                            (:1
                              (Variables|/Game/Blueprints/CharacterBP/bp_baseCharacter.bp_baseCharacter_C|SetdashInput _user_2 "NewEnumerator2"))
                            (:2
                              (Variables|/Game/Blueprints/CharacterBP/bp_baseCharacter.bp_baseCharacter_C|SetdashInput _user_2 "NewEnumerator3"))
                            (:3
                              (Variables|Default|SetnextAction "NewEnumerator5")))
                          (Variables|Default|SetnextAction "NewEnumerator6"))))
                    (:NewEnumerator7
                      (if (> (Variables|/Game/Blueprints/CharacterBP/bp_baseCharacter.bp_baseCharacter_C|GetcurrentHealth _user_2) (Math|Float|Round (* (Math|Conversions|ToFloat(Integer) (Variables|/Game/Blueprints/CharacterBP/bp_baseCharacter.bp_baseCharacter_C|GetMaxHealth _user_2)) 0.5)))
                        (switch int (Math|Random|RandomIntegerinRange 0 2) :!label _label
                          (:0
                            (Variables|Default|SetnextAction "NewEnumerator5"))
                          (:1
                            (Variables|/Game/Blueprints/CharacterBP/bp_baseCharacter.bp_baseCharacter_C|SetdashInput (Variables|Default|GetUser) "NewEnumerator0" :!label _label_2)
                            (Variables|Default|SetnextAction "NewEnumerator6"))
                          (:2
                            (goto _label_2)))
                        (else
                          (Variables|Default|SetnextAction "NewEnumerator7"))))
                    (:NewEnumerator8
                      (goto _label))
                    (:NewEnumerator9
                      (Variables|/Game/Blueprints/CharacterBP/bp_baseCharacter.bp_baseCharacter_C|SetdashInput (Variables|Default|GetUser) "NewEnumerator0" :!label _label_3)
                      (Variables|Default|SetnextAction "NewEnumerator6"))
                    (:NewEnumerator10
                      (goto _label_3))))
                (else
                  (switch Utilities|FlowControl|Switch|SwitchonStates (Variables|/Game/Blueprints/CharacterBP/bp_baseCharacter.bp_baseCharacter_C|GetcurrentState (Variables|Default|GetUser))
                    (:NewEnumerator3
                      (Variables|Default|SetnextAction "NewEnumerator3"))
                    (:NewEnumerator4
                      (Variables|Default|SetnextAction "NewEnumerator4"))
                    (:NewEnumerator5
                      (switch int (Math|Random|RandomIntegerinRange 0 1)
                        (:0
                          (Variables|Default|SetnextAction "NewEnumerator5"))
                        (:1
                          (Variables|/Game/Blueprints/CharacterBP/bp_baseCharacter.bp_baseCharacter_C|SetdashInput _user_3 "NewEnumerator0")
                          (Variables|Default|SetnextAction "NewEnumerator6"))))
                    (:NewEnumerator6
                      (switch Utilities|FlowControl|Switch|SwitchonInput_Enums (Variables|/Game/Blueprints/CharacterBP/bp_baseCharacter.bp_baseCharacter_C|GetdashInput _user_3)
                        (:NewEnumerator0
                          (Utilities|FlowControl|Delay (Math|Random|RandomFloatinRange (Variables|Default|GetWaitMin) (Variables|Default|GetWaitMax)))
                          (if (Variables|/Game/Blueprints/CharacterBP/bp_baseCharacter.bp_baseCharacter_C|GetAttackSnap_inRange _user_5)
                            (switch int (Math|Random|RandomIntegerinRange 0 1)
                              (:0
                                (Variables|Default|SetnextAction "NewEnumerator3"))
                              (:1
                                (Variables|Default|SetnextAction "NewEnumerator4")))
                            (else
                              (switch int (Math|Random|RandomIntegerinRange 0 1)
                                (:0
                                  (Variables|/Game/Blueprints/CharacterBP/bp_baseCharacter.bp_baseCharacter_C|SetdashInput _user_5 "NewEnumerator0")
                                  (Variables|Default|SetnextAction "NewEnumerator6"))
                                (:1
                                  (Variables|Default|SetnextAction "NewEnumerator5"))))))))
                    (:NewEnumerator7
                      (Variables|/Game/Blueprints/CharacterBP/bp_baseCharacter.bp_baseCharacter_C|SetdashInput _user_3 "NewEnumerator1")
                      (Variables|Default|SetnextAction "NewEnumerator6"))
                    (:NewEnumerator9
                      (switch int (Math|Random|RandomIntegerinRange 0 1) :!label _label_4
                        (:0
                          (Utilities|FlowControl|Delay (Math|Random|RandomFloatinRange 0.0 5.0))
                          (Default|AerialRecoveryLogic _user_6)
                          (Variables|/Game/Blueprints/CharacterBP/bp_baseCharacter.bp_baseCharacter_C|SetdashInput _user_6 "NewEnumerator1")
                          (Variables|Default|SetnextAction "NewEnumerator6"))
                        (:1
                          (Variables|Default|SetnextAction "NewEnumerator0"))))
                    (:NewEnumerator10
                      (goto _label_4))
                    (:NewEnumerator11
                      (switch int (Math|Random|RandomIntegerinRange 0 2)
                        (:0
                          (Variables|Default|SetnextAction "NewEnumerator3"))
                        (:1
                          (Variables|/Game/Blueprints/CharacterBP/bp_baseCharacter.bp_baseCharacter_C|SetdashInput (Variables|Default|GetUser) "NewEnumerator1")
                          (Variables|Default|SetnextAction "NewEnumerator6"))
                        (:2
                          (Variables|Default|SetnextAction "NewEnumerator8")))))))
              (else
                ;[1 1 1] nextActionInQue
                (switch Utilities|FlowControl|Switch|SwitchonStates (Variables|Default|GetnextAction)
                  (:NewEnumerator3
                    (Default|LATKLogic _user_4))
                  (:NewEnumerator4
                    (Default|HATKLogic _user_4))
                  (:NewEnumerator5
                    (Default|ProjectileLogic _user_4))
                  (:NewEnumerator6
                    (Variables|/Game/Blueprints/CharacterBP/bp_baseCharacter.bp_baseCharacter_C|SetcurrentState _user_4 "NewEnumerator6")
                    (switch Utilities|FlowControl|Switch|SwitchonInput_Enums (Variables|/Game/Blueprints/CharacterBP/bp_baseCharacter.bp_baseCharacter_C|GetdashInput _user_4)
                      (:NewEnumerator0
                        (if (Variables|/Game/Blueprints/CharacterBP/bp_baseCharacter.bp_baseCharacter_C|GetDashSnap_inRange _user_4)
                          (Default|DashSnap _user_4)
                          (else
                            (Default|DashForward _user_4))))
                      (:NewEnumerator1
                        (Default|DashBack _user_4))
                      (:NewEnumerator2
                        (Default|DashLeft _user_4))
                      (:NewEnumerator3
                        (Default|DashRight _user_4))))
                  (:NewEnumerator7
                    (Default|HealLogic _user_4))
                  (:NewEnumerator8
                    (Default|BlockLogic _user_4)))
                (Variables|Default|SetnextAction "NewEnumerator0")))
            (else
              (Utilities|FlowControl|Delay (Math|Random|RandomFloatinRange 0.0 5.0))
              (Default|KnockedDownGetUp (Variables|Default|GetUser)))))))))

(fn ConstructionScript)

(fn CheckUserIdle
  (if (Utilities|Enum|Equal(Enum) (Variables|/Game/Blueprints/CharacterBP/bp_baseCharacter.bp_baseCharacter_C|GetcurrentState (Variables|Default|GetUser)) "NewEnumerator0")
    (return true)
    (else
      (return false))))

(fn CheckUserKnockedDown
  (if (Utilities|Enum|Equal(Enum) (Variables|/Game/Blueprints/CharacterBP/bp_baseCharacter.bp_baseCharacter_C|GetcurrentState (Variables|Default|GetUser)) "NewEnumerator12")
    (return true)
    (else
      (return false))))