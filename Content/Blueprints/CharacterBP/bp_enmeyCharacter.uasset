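; Enemy character Blueprint that publishes its world position as the boss location for other systems to read.
; On BeginPlay, it starts a very fast looping function-name timer, unless it is the pawn controlled by player 0.
; Each timer call casts to the gameInfo_instance game instance and writes the actor's location into BossLocation, avoiding Tick.
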(event EventBeginPlay
  (|CallParentFunction)
  (CallFunction|CallSendLocationLoop))

(event Collision|EventActorBeginOverlap
  (params (OtherActor :type Actor%20Object%20Reference)))

(event EventTick
  (params (DeltaSeconds :type Float%20%28single-precision%29))
  (|CallParentFunction DeltaSeconds) ; This node is disabled and will not be called.\nDrag off pins to build functionality.
)

(fn ConstructionScript
  (|CallParentFunction))

(fn SendLocation
  (bind _asgame_info_instance (Utilities|Casting|CastTogameInfo_instance (Game|GetGameInstance)))
  (Variables|/Game/Blueprints/Instance/gameInfo_instance.gameInfo_instance_C|SetbossLocation _asgame_info_instance (Transformation|GetActorLocation)))

(fn CallSendLocationLoop
  (if (not (== self (Pawn|GetControlledPawn (Game|GetPlayerController 0))))
    (Utilities|Time|SetTimerbyFunctionName 0 "sendLocation" 0.005 true)))