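; Interactable pickup actor that the player can pick up and drop back into the world.
; On interaction it asks the player to pick it up and, if that succeeds, disables its own collision.
; DropItem traces straight down on the Visibility channel, ignoring the player, and on a hit re-enables collision, detaches and moves to the hit point.
; It returns whether a surface was found.
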(event EventBeginPlay
  (|CallParentFunction) ; This node is disabled and will not be called.\nDrag off pins to build functionality.
)

(event Collision|EventActorBeginOverlap
  (params (OtherActor :type Actor%20Object%20Reference))
  (|CallParentFunction OtherActor) ; This node is disabled and will not be called.\nDrag off pins to build functionality.
)

(event EventTick
  (params (DeltaSeconds :type Float%20%28single-precision%29))
  (|CallParentFunction DeltaSeconds) ; This node is disabled and will not be called.\nDrag off pins to build functionality.
)

(event EventInteraction
  (|CallParentFunction)
  (bind _isattached (Default|PickupItem (Variables|Default|GetPlayer) self))
  (if _isattached
    (Collision|SetActorEnableCollision false)))

(fn ConstructionScript
  (|CallParentFunction))

(fn DropItem
  (bind _returnvalue (Transformation|GetActorLocation))
  (bind (_outhit _returnvalue_2) (Collision|LineTraceByChannel _returnvalue (+ _returnvalue (Math|Vector|MakeVector 0.0 0.0 -2e+03)) "TraceTypeQuery1" false (Utilities|Array|MakeArray (Variables|Default|GetPlayer)) "None"))
  (if _returnvalue_2
    (Collision|SetActorEnableCollision true)
    (Transformation|DetachFromActor "KeepRelative" "KeepRelative" "KeepRelative")
    (Transformation|SetActorLocationAndRotation (.Location (Collision|BreakHitResult _outhit)) "0, 0, 0"))
  (return _returnvalue_2))