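; Base interactable actor that registers itself with GarrettsPawn while the pawn overlaps its sphere trigger, leaving Interaction empty.
; The construction script applies configurable mesh, scale, offsets and trigger radius to its components.
; BeginPlay sets the description on the widget component and creates a separate WBP_Interact_UI instance.
; ToggleHighlight shows or hides both, adding the created widget to the viewport only once.
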(event OnComponentBeginOverlap(InteractionTrigger)
  (params (OverlappedComponent :type Primitive%20Component%20Object%20Reference) (OtherActor :type Actor%20Object%20Reference) (OtherComp :type Primitive%20Component%20Object%20Reference) (OtherBodyIndex :type Integer) (bFromSweep :type Boolean) (SweepResult :type Hit%20Result%20Structure%20%28by%20ref%29))
  (bind _asgarretts_pawn (Utilities|Casting|CastToGarrettsPawn OtherActor))
  (bind _output_get (Variables|Default|SetPlayer _asgarretts_pawn))
  (Default|AddInteraction _output_get self))

(event OnComponentEndOverlap(InteractionTrigger)
  (params (OverlappedComponent :type Primitive%20Component%20Object%20Reference) (OtherActor :type Actor%20Object%20Reference) (OtherComp :type Primitive%20Component%20Object%20Reference) (OtherBodyIndex :type Integer))
  (bind _asgarretts_pawn (Utilities|Casting|CastToGarrettsPawn OtherActor))
  (bind _output_get (Variables|Default|SetPlayer _asgarretts_pawn))
  (Default|RemoveInteraction _output_get self))

(event EventBeginPlay
  (CallFunction|SetupUIText)
  (bind _returnvalue (UserInterface|CreateWidget "/Game/Blueprints/InteractableObjects/WBP_Interact_UI.WBP_Interact_UI_C"))
  (Variables|Default|SetUI _returnvalue))

(event Collision|EventActorBeginOverlap
  (params (OtherActor :type Actor%20Object%20Reference)))

(event EventTick
  (params (DeltaSeconds :type Float%20%28single-precision%29)))

(fn ConstructionScript
  (CallFunction|SetupInteractionUI)
  (CallFunction|SetupInteractionTrigger)
  (CallFunction|SetupMesh))

(fn ToggleHighlight
  (params (Highlight :type Boolean))
  (bind _ui (Variables|Default|GetUI))
  (Rendering|SetVisibility (Variables|Default|GetInteractionUI) Highlight false)
  (if Highlight
    (Utilities|FlowControl|Sequence
      (:then_0
        (Utilities|FlowControl|DoOnce false
          (:Completed
            (UserInterface|Viewport|AddtoViewport _ui 1))))
      (:then_1
        (Widget|SetVisibility _ui "Visible")))
    (else
      (Widget|SetVisibility _ui "Hidden"))))

(fn Interaction)

(fn SetupInteractionUI
  (Transformation|SetRelativeLocation (Variables|Default|GetInteractionUI) (Variables|Default|GetUIOffset) false false))

(fn SetupUIText
  (bind _aswbp_interact_ui (Utilities|Casting|CastToWBP_Interact_UI (UserInterface|GetUserWidgetObject (Variables|Default|GetInteractionUI))))
  (Default|SetInteractionText _aswbp_interact_ui (Variables|Default|GetUIDescription)))

(fn SetupInteractionTrigger
  (Components|Sphere|SetSphereRadius (Variables|Default|GetInteractionTrigger) (Variables|Default|GetTriggerRadius) true)
  (Transformation|SetRelativeLocation (Variables|Default|GetInteractionTrigger) (Variables|Default|GetTriggerOffset) false false))

(fn SetupMesh
  (Components|StaticMesh|SetStaticMesh (Variables|Default|GetInteractionMesh) (Variables|Default|GetActorMesh))
  (Transformation|SetRelativeLocation (Variables|Default|GetInteractionMesh) (Variables|Default|GetMeshOffset) false false)
  (Transformation|SetWorldScale3D (Variables|Default|GetInteractionMesh) (Variables|Default|GetMeshScale)))