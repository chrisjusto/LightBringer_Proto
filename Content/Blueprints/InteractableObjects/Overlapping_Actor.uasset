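; Interactable actor with a mesh and three sphere trigger points, apparently meant to start a boss sequence once the points are matched.
; Construction sets the mesh, shared sphere radius and each point's offset.
; Overlap events set a flag per point when the other component carries that point's tag, clearing it on exit.
; Tick compares the flags by chained equality rather than AND, and its branch is still empty.
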(event OnComponentBeginOverlap(Point1)
  (params (OverlappedComponent :type Primitive%20Component%20Object%20Reference) (OtherActor :type Actor%20Object%20Reference) (OtherComp :type Primitive%20Component%20Object%20Reference) (OtherBodyIndex :type Integer) (bFromSweep :type Boolean) (SweepResult :type Hit%20Result%20Structure%20%28by%20ref%29))
  (bind _iscolliding (CallFunction|CheckPoints OtherComp "Point1"))
  (Variables|Default|SetPoint_1_Collision _iscolliding))

(event OnComponentBeginOverlap(Point2)
  (params (OverlappedComponent :type Primitive%20Component%20Object%20Reference) (OtherActor :type Actor%20Object%20Reference) (OtherComp :type Primitive%20Component%20Object%20Reference) (OtherBodyIndex :type Integer) (bFromSweep :type Boolean) (SweepResult :type Hit%20Result%20Structure%20%28by%20ref%29))
  (bind _iscolliding (CallFunction|CheckPoints OtherComp "Point2"))
  (Variables|Default|SetPoint_2_Collision _iscolliding))

(event OnComponentBeginOverlap(Point3)
  (params (OverlappedComponent :type Primitive%20Component%20Object%20Reference) (OtherActor :type Actor%20Object%20Reference) (OtherComp :type Primitive%20Component%20Object%20Reference) (OtherBodyIndex :type Integer) (bFromSweep :type Boolean) (SweepResult :type Hit%20Result%20Structure%20%28by%20ref%29))
  (bind _iscolliding (CallFunction|CheckPoints OtherComp "Point3"))
  (Variables|Default|SetPoint_3_Collision _iscolliding))

(event OnComponentEndOverlap(Point1)
  (params (OverlappedComponent :type Primitive%20Component%20Object%20Reference) (OtherActor :type Actor%20Object%20Reference) (OtherComp :type Primitive%20Component%20Object%20Reference) (OtherBodyIndex :type Integer))
  (Variables|Default|SetPoint_1_Collision false))

(event OnComponentEndOverlap(Point2)
  (params (OverlappedComponent :type Primitive%20Component%20Object%20Reference) (OtherActor :type Actor%20Object%20Reference) (OtherComp :type Primitive%20Component%20Object%20Reference) (OtherBodyIndex :type Integer))
  (Variables|Default|SetPoint_2_Collision false))

(event OnComponentEndOverlap(Point3)
  (params (OverlappedComponent :type Primitive%20Component%20Object%20Reference) (OtherActor :type Actor%20Object%20Reference) (OtherComp :type Primitive%20Component%20Object%20Reference) (OtherBodyIndex :type Integer))
  (Variables|Default|SetPoint_3_Collision false))

(event EventBeginPlay)

(event Collision|EventActorBeginOverlap
  (params (OtherActor :type Actor%20Object%20Reference)))

(event EventTick
  (params (DeltaSeconds :type Float%20%28single-precision%29))
  ;[1 1 1] If true, do boss sequence
  (if (Math|Boolean|Equal(Boolean) (Math|Boolean|Equal(Boolean) (Variables|Default|GetPoint_1_Collision) (Variables|Default|GetPoint_2_Collision)) (Variables|Default|GetPoint_3_Collision))
    _))

(fn ConstructionScript
  (CallFunction|SetupMesh)
  (CallFunction|SetCollisionScale)
  (CallFunction|SetPoint1Location)
  (CallFunction|SetPoint2Location)
  (CallFunction|SetPoint3Location))

(fn SetupMesh
  (Components|StaticMesh|SetStaticMesh (Variables|Default|GetMesh) (Variables|Default|GetActor_Mesh)))

(fn SetCollisionScale
  (Components|Sphere|SetSphereRadius (Variables|Default|GetPoint1) (Variables|Default|GetCollision_Radius) true))

(fn SetPoint1Location
  (Transformation|AddLocalOffset (Variables|Default|GetPoint1) (Variables|Default|GetPoint_1_Location) false false))

(fn SetPoint2Location
  (Transformation|AddLocalOffset (Variables|Default|GetPoint2) (Variables|Default|GetPoint_2_Location) false false))

(fn SetPoint3Location
  (Transformation|AddLocalOffset (Variables|Default|GetPoint3) (Variables|Default|GetPoint_3_Location) false false))

(fn CheckPoints
  (params (Point :type Primitive%20Component%20Object%20Reference) (Tag :type Name))
  (bind _returnvalue (Components|ComponentHasTag Point Tag))
  (if _returnvalue
    (return _returnvalue)
    (else
      (return _returnvalue))))